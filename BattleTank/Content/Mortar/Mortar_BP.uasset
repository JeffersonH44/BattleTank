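; Mortar Blueprint that reuses the TankAiming component to aim a mortar made of a dome and a barrel.
; The construction script assigns the dome and barrel meshes and sets Projectile_BP as the component's projectile class.
; On BeginPlay it initializes TankAiming with the barrel and with the dome as the turret.
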(event `self.ReceiveBeginPlay`
  (`TankAimingComponent.Initialize` (`self.TankAiming`) (`self.MortarBarrel`) (`self.MortarDome`)))

(fn `UserConstructionScript`
  (set `TankAimingComponent.ProjectileBlueprint` "/Game/Tank/Projectile_BP.Projectile_BP_C" (`self.TankAiming`))
  (`StaticMeshComponent.SetStaticMesh` (`self.MortarDome`) "/Game/Mortar/mortar_dome.mortar_dome")
  (`StaticMeshComponent.SetStaticMesh` (`self.MortarBarrel`) "/Game/Mortar/mortar_barrel.mortar_barrel"))